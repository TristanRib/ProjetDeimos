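; BPC_Damageable_Child is a damageable component Blueprint in the damage system, with logic for health, blocking and death.
; CanBeDamaged routes a damage info to receive, block or no-damage exits using dead, invincibility and blocking states plus the hit's flags.
; ReceiveDamage_0 only returns false: its block callback, health subtraction, death and hit-effect branches are disconnected, and nothing here calls CanBeDamaged.
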(fn ReceiveDamage0
  (params (DamageInfo :type S%20Damage%20Info%20Structure))
  (return false))