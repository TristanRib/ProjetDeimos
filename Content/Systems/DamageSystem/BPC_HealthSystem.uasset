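; Health component that tracks current and max health, death state, and responses to incoming damage.
; ReceiveDamage routes hits through a CanBeDamaged macro that checks death, invincibility and blocking, then fires death, hit-effect or blocked dispatchers.
; Heal and direct health setters clamp to the valid range, while ReceiveDamage subtracts unclamped.
; Add and Reduce Max Health assign the given value outright and broadcast it; ReduceHealth broadcasts only at zero, without calling OnDeath.
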(fn SetMaxHealth
  (params (Health :type Float%20%28double-precision%29))
  (bind _output_get (Variables|Health|SetMaxHealth Health))
  (Variables|Health|SetCurrentHealth (Math|Float|Clamp(Float) (Variables|Health|GetCurrentHealth) 0.0 _output_get)))

(fn GetMaxHealth
  (return (Variables|Health|GetMaxHealth)))

(fn SetCurrentHealth
  (params (Health :type Float%20%28double-precision%29))
  (Variables|Health|SetCurrentHealth (Math|Float|Clamp(Float) Health 0.0 (Variables|Health|GetMaxHealth))))

(fn GetCurrentHealth
  (return (Variables|Health|GetCurrentHealth)))

(fn Heal
  (params (Amount :type Float%20%28double-precision%29))
  (if (not (Variables|Health|GetIsDead))
    (Variables|Health|SetCurrentHealth (Math|Float|Clamp(Float) (+ Amount (Variables|Health|GetCurrentHealth)) 0.0 (Variables|Health|GetMaxHealth)))
    (return 0.0)))

(fn ReceiveDamage
  (params (DamageInfo :type S%20Damage%20Info%20Structure))
  (bind (_damageamount _hittype _damagetype _isblockable _isparryable) (Utilities|Struct|BreakS_DamageInfo DamageInfo))
  (Utilities|CanbeDamaged DamageInfo
    (:NoDamage
      (return false))
    (:ReceiveDamage
      (bind _output_get (Variables|Health|SetCurrentHealth (- (Variables|Health|GetCurrentHealth) _damageamount)))
      (if (<= _output_get 0.0)
        (Variables|Health|SetIsDead true)
        (Default|CallOnDeath)
        (else
          (Default|CallOnHitEffect _hittype)))
      (return true))
    (:BlockDamage
      (Default|CallOnBlocked _isparryable)
      (return false))))

(fn AddMaxHealth
  (params (Value :type Float%20%28double-precision%29))
  (bind _output_get (Variables|Health|SetMaxHealth Value))
  (Default|CallOnMaxHealthUpdated _output_get)
  (return _output_get))

(fn ReduceMaxHealth
  (params (Value :type Float%20%28double-precision%29))
  (bind _output_get (Variables|Health|SetMaxHealth Value))
  (Variables|Health|SetCurrentHealth (Math|Float|Clamp(Float) (Variables|Health|GetCurrentHealth) 0.0 _output_get))
  (Default|CallOnMaxHealthUpdated (Variables|Health|GetMaxHealth))
  (return (Variables|Health|GetMaxHealth)))

(fn ReceiveInteraction)

(fn AddHealth
  (params (Value :type Float%20%28double-precision%29))
  (bind _output_get (Variables|Health|SetCurrentHealth (Math|Float|Clamp(Float) (+ (Variables|Health|GetCurrentHealth) Value) 0.0 (Variables|Health|GetMaxHealth))))
  (Default|CallOnHealthUpdated _output_get)
  (return _output_get))

(fn ReduceHealth
  (params (Value :type Float%20%28double-precision%29))
  (bind _output_get (Variables|Health|SetCurrentHealth (Math|Float|Clamp(Float) (- (Variables|Health|GetCurrentHealth) Value) 0.0 (Variables|Health|GetMaxHealth))))
  (if (== _output_get 0.0)
    (bind _output_get_2 (Variables|Health|SetIsDead true))
    (Default|CallOnHealthUpdated (Variables|Health|GetCurrentHealth)))
  (return (Variables|Health|GetCurrentHealth) _output_get_2))

(fn GetIsDead
  (return (Variables|Health|GetIsDead)))