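; BPC_Damageable_Child is a health-system component that decides whether incoming damage applies.
; ReceiveDamage runs the CanBeDamaged macro on DamageInfo, updates health on success and returns whether damage landed.
; Damage passes while health is above zero, or regardless when it ignores invincibility.
; A block exit exists, but its hardcoded false condition keeps it from firing, and the invincibility check likewise uses a constant.
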(fn ReceiveDamage
  (params (DamageInfo :type S%20Damage%20Info%20Structure))
  (Utilities|CanbeDamaged DamageInfo
    (:NoDamage
      _)
    (:ReceiveDamage
      (CallFunction|UpdateHealth (.DamageAmount (Utilities|Struct|BreakS_DamageInfo DamageInfo)))
      (return true))
    (:BlockDamage
      _))
  (return false))