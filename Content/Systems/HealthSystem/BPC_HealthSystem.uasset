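; Actor component that tracks an actor's Health and MaxHealth and broadcasts change events carrying new and previous values.
; Setters clamp Health to MaxHealth and fire Updated plus Increased or Decreased dispatchers only on actual change.
; The component listens to its own dispatchers to raise zero and full health events and lower Health when MaxHealth drops below it.
; Additive Update functions ignore zero amounts and do nothing once Health is zero.
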(event Custom|HealthDecreasedEvent
  (params (Info :type S%20Health%20Change%20Info%20Structure))
  ;[0.15 0.15 0.15 0.5] Check after each Health decrease if OnZeroHealth event should be triggered
  (bind _returnvalue (HealthSystem|IsZeroHealth))
  (if _returnvalue
    (Default|CallOnZeroHealth)))

(event Custom|HealthIncreasedEvent
  (params (Info :type S%20Health%20Change%20Info%20Structure))
  ;[0.15 0.15 0.15 0.5] Check after each Health increase if OnFullHealth event should be triggered
  (bind _returnvalue (HealthSystem|IsFullHealth))
  (if _returnvalue
    (Default|CallOnFullHealth)))

(event Custom|MaxHealthDecreasedEvent
  (params (Info :type S%20Health%20Change%20Info%20Structure))
  (bind _newvalue (Utilities|Struct|BreakS_HealthChangeInfo Info))
  ;[0.15 0.15 0.15 0.5] Check after each MaxHealth decrease if Health should be decreased accordingly
  (if (< _newvalue (Variables|HealthSystem|GetHealth))
    (HealthSystem|SetHealth _newvalue)))

(event EventBeginPlay
  ;[0.15 0.15 0.15 0.5] Events binding
  (EventDispatchers|BindEventtoOnHealthDecreased (EventDispatchers|CreateEvent :!event Custom|HealthDecreasedEvent))
  (EventDispatchers|BindEventtoOnHealthIncreased (EventDispatchers|CreateEvent :!event Custom|HealthIncreasedEvent))
  (EventDispatchers|BindEventtoOnMaxHealthDecreased (EventDispatchers|CreateEvent :!event Custom|MaxHealthDecreasedEvent)))

(fn SetMaxHealth
  (params (MaxHealth :type Float%20%28double-precision%29))
  (if (> MaxHealth (Variables|HealthSystem|GetMaxHealth))
    (Utilities|FlowControl|Sequence
      (:then_0
        (bind _output_get (Variables|HealthSystem|SetMaxHealth MaxHealth :!label _label))
        (Default|CallOnMaxHealthUpdated (Utilities|Struct|MakeS_HealthChangeInfo _output_get (Variables|HealthSystem|GetMaxHealth) 0)))
      (:then_1
        (Default|CallOnMaxHealthIncreased (Utilities|Struct|MakeS_HealthChangeInfo _output_get (Variables|HealthSystem|GetMaxHealth) 0))))
    (elif (< MaxHealth (Variables|HealthSystem|GetMaxHealth))
      (Utilities|FlowControl|Sequence
        (:then_0
          (goto _label))
        (:then_1
          (Default|CallOnMaxHealthDecreased (Utilities|Struct|MakeS_HealthChangeInfo _output_get (Variables|HealthSystem|GetMaxHealth) 0)))))))

(fn GetMaxHealth
  (return (Variables|HealthSystem|GetMaxHealth)))

(fn UpdateMaxHealth
  (params (Amount :type Float%20%28double-precision%29))
  (bind _returnvalue (HealthSystem|IsZeroHealth))
  (if (not (or _returnvalue (== Amount 0.0)))
    (HealthSystem|SetMaxHealth (+ (Variables|HealthSystem|GetMaxHealth) Amount))))

(fn SetHealth
  (params (Health :type Float%20%28double-precision%29))
  (bind _output_get (LocalVariables|SetNewValue (Math|Float|Clamp(Float) Health 0.0 (Variables|HealthSystem|GetMaxHealth))))
  (if (> _output_get (Variables|HealthSystem|GetHealth))
    (Utilities|FlowControl|Sequence
      (:then_0
        (LocalVariables|SetPreviousValue (Variables|HealthSystem|GetHealth) :!label _label)
        (Variables|HealthSystem|SetHealth (LocalVariables|GetNewValue))
        (Default|CallOnHealthUpdated (Utilities|Struct|MakeS_HealthChangeInfo (LocalVariables|GetNewValue) (LocalVariables|GetPreviousValue) 0)))
      (:then_1
        (Default|CallOnHealthIncreased (Utilities|Struct|MakeS_HealthChangeInfo (LocalVariables|GetNewValue) (LocalVariables|GetPreviousValue) 0))))
    (elif (< _output_get (Variables|HealthSystem|GetHealth))
      (Utilities|FlowControl|Sequence
        (:then_0
          (goto _label))
        (:then_1
          (Default|CallOnHealthDecreased (Utilities|Struct|MakeS_HealthChangeInfo (LocalVariables|GetNewValue) (LocalVariables|GetPreviousValue) 0)))))))

(fn GetHealth
  (return (Variables|HealthSystem|GetHealth)))

(fn UpdateHealth
  (params (Amount :type Float%20%28double-precision%29))
  (bind _returnvalue (HealthSystem|IsZeroHealth))
  (if (not (or _returnvalue (== 0.0 Amount)))
    (HealthSystem|SetHealth (+ (Variables|HealthSystem|GetHealth) Amount))))

(fn GetHealthPercentage
  (return (Math|Float|SafeDivide (Variables|HealthSystem|GetHealth) (Variables|HealthSystem|GetMaxHealth))))

(fn IsFullHealth
  (return (== (Variables|HealthSystem|GetMaxHealth) (Variables|HealthSystem|GetHealth))))

(fn IsZeroHealth
  (return (== (Variables|HealthSystem|GetHealth) 0.0)))