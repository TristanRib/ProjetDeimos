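; Stamina component that stores a current and maximum stamina value for its owner.
; SetStamina clamps to zero and max, then broadcasts updated and directional change events with previous and new values, though Increased and Decreased appear swapped relative to the comparisons.
; UpdateStamina applies non-zero deltas through SetStamina, alongside getters and full/empty checks.
; SetMaxStamina and UpdateMaxStamina are empty stubs, and no Tick logic runs.
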(event EventBeginPlay)

(event EventTick
  (params (DeltaSeconds :type Float%20%28single-precision%29)))

(fn GetStamina
  (return (Variables|StaminaSystem|GetStamina)))

(fn SetStamina
  (params (Stamina :type Float%20%28double-precision%29))
  (bind _output_get (LocalVariables|SetNew%20Value (Math|Float|Clamp(Float) Stamina 0.0 (Variables|StaminaSystem|GetMaxStamina))))
  (if (< _output_get (Variables|StaminaSystem|GetStamina))
    (Utilities|FlowControl|Sequence
      (:then_0
        (LocalVariables|SetPrevious%20value (Variables|StaminaSystem|GetStamina) :!label _label)
        (Variables|StaminaSystem|SetStamina (LocalVariables|GetNew%20Value))
        (Default|CallOnStaminaUpdated (Utilities|Struct|MakeS_StaminaChangeInfo (LocalVariables|GetPrevious%20value) (LocalVariables|GetNew%20Value))))
      (:then_1
        (Default|CallOnStaminaIncreased (Utilities|Struct|MakeS_StaminaChangeInfo (LocalVariables|GetPrevious%20value) (LocalVariables|GetNew%20Value)))))
    (elif (> _output_get (Variables|StaminaSystem|GetStamina))
      (Utilities|FlowControl|Sequence
        (:then_0
          (goto _label))
        (:then_1
          (Default|CallOnStaminaDecreased (Utilities|Struct|MakeS_StaminaChangeInfo (LocalVariables|GetPrevious%20value) (LocalVariables|GetNew%20Value))))))))

(fn UpdateStamina
  (params (Amount :type Float%20%28double-precision%29))
  (if (not (== 0.0 Amount))
    (StaminaSystem|SetStamina (+ Amount (Variables|StaminaSystem|GetStamina)))))

(fn GetMaxStamina
  (return (Variables|StaminaSystem|GetMaxStamina)))

(fn SetMaxStamina)

(fn UpdateMaxStamina)

(fn IsFullStamina
  (return (== (Variables|StaminaSystem|GetMaxStamina) (Variables|StaminaSystem|GetStamina))))

(fn IsZeroStamina
  (return (== 0.0 (Variables|StaminaSystem|GetStamina))))