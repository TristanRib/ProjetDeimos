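; BPC_InventorySystem is a Blueprint inventory component that holds an array of item slots.
; On BeginPlay it calls SetupSlotsSERVER, intended for the server, which fills ItemSlots with SlotsAmount slot structs, each storing its index and a reference back to the component.
; AddItem is a stub that always returns false.
; FindEmptySlot is unfinished, returning true on the first slot without checking whether it is empty.
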(event Custom|SetupSlotsSERVER
  (params (SlotsAmount :type Integer))
  ;[0.15 0.15 0.15 0.5] Setup Inventory Slot on Server
  (bind _output_get (Variables|InventorySystem|SetSlotsAmount SlotsAmount))
  (for _index (range 0 (- _output_get 1))
    (Utilities|Array|Add (Variables|InventorySystem|GetItemSlots) (Utilities|Struct|MakeS_InventorySlot _index self))))

(event EventBeginPlay
  (CallFunction|SetupSlotsSERVER (Variables|InventorySystem|GetSlotsAmount)))

(fn AddItem
  (params (ItemToAdd :type S%20Inventory%20Slot%20Structure))
  (return false))

(fn FindEmptySlot
  (for _array_element (Variables|InventorySystem|GetItemSlots)
    (if true
      (return true ""))))