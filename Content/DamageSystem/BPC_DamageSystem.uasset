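; BPC_DamageSystem is a damage component that handles health, healing, blocking and death.
; ReceiveDamage runs incoming damage info through the CanBeDamaged macro, which uses death, invincibility and blocking state to pick no damage, damage or block.
; Damage lowers health, then fires death or hit-effect dispatchers, while blocks fire a blocked dispatcher with parry info.
; Heal restores health up to the maximum unless dead.
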(event EventBeginPlay)

(event EventTick
  (params (DeltaSeconds :type Float%20%28single-precision%29)))

(fn Heal
  (params (Amount :type Float%20%28double-precision%29))
  (if (not (Variables|Default|GetIsDead))
    (Variables|Default|SetCurrentHealth (Math|Float|Clamp(Float) (+ Amount (Variables|Default|GetCurrentHealth)) 0.0 (Variables|Default|GetMaxHealth)))
    (return 0.0)))

(fn ReceiveDamage
  (params (DamageInfo :type S%20Damage%20Info%20Structure))
  (bind (_damageamount _hittype _damagetype _isblockable _isparryable) (Utilities|Struct|BreakS_DamageInfo DamageInfo))
  (Utilities|CanbeDamaged DamageInfo
    (:NoDamage
      (return false))
    (:ReceiveDamage
      (bind _output_get (Variables|Default|SetCurrentHealth (- (Variables|Default|GetCurrentHealth) _damageamount)))
      (if (<= _output_get 0.0)
        (Variables|Default|SetIsDead true)
        (Default|CallOnDeath)
        (else
          (Default|CallOnHitEffect _hittype)))
      (return true))
    (:BlockDamage
      (Default|CallOnBlocked _isparryable)
      (return false))))