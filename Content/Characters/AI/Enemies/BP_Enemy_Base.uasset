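; BP_Enemy_Base is a base enemy character with health, a push/shove attack and speed control for AI use.
; Damage lowers health and launches the character along the causer's forward vector with some lift, then turns the mesh into a ragdoll at zero health.
; Alerts are forwarded to the cached AIC_Enemy_Base controller as heard locations, while Attack plays a montage and signals its end.
; Helper functions supply attack and defend ranges and map movement states to walk speeds.
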(event Custom|Attack
  ;[1 1 1] Behavior
  ;;[0.05127 0.05127 0.05127] Attack
  (Animation|Montage|PlayMontage (Variables|Character|GetMesh) "/Game/Characters/Mannequin_UE4/Animations/Paired_PushShove_Att_Montage.Paired_PushShove_Att_Montage"
    (:OnCompleted
      _)
    (:OnInterrupted
      _))
  (Default|CallOnAttackEnd))

(event EventAlertSurrounding
  (params (Target :type Object%20Object%20Reference) (Location :type Vector :default "0, 0, 0"))
  ;[1 1 1] Behavior
  ;;[0.05127 0.05127 0.05127] As been alerted
  (bind _asaic_enemy_base (Utilities|Casting|CastToAIC_Enemy_Base (Variables|Default|GetAI%20Controller)))
  (Default|HandleSensedHearing _asaic_enemy_base Location))

(event EventBeginPlay
  ;[1 1 1] setup
  (Variables|Default|SetAI%20Controller (AI|GetAIController self)))

(event Game|Damage|EventAnyDamage
  (params (Damage :type Float%20%28single-precision%29) (DamageType :type Damage%20Type%20Object%20Reference) (InstigatedBy :type Controller%20Object%20Reference) (DamageCauser :type Actor%20Object%20Reference))
  ;[1 0 0] Health system
  (bind _output_get (Variables|Default|SetHealth (- (Variables|Default|GetHealth) Damage)))
  (if (Utilities|IsValid DamageCauser)
    (Character|LaunchCharacter (+ (* (Transformation|GetActorForwardVector DamageCauser) 2e+02) (* (Transformation|GetActorUpVector) 1e+02)) false false))
  (if (<= _output_get 0.0)
    (Physics|SetSimulatePhysics (Variables|Character|GetMesh) true)))

(fn ConstructionScript)

(fn GetIdealRange
  (return 1.5e+02 3.5e+02))

(fn SetMovementSpeed
  (params (Speed :type E_MovementSpeed%20Enum :default "NewEnumerator0"))
  (bind _output_get (Variables|/Script/Engine.CharacterMovementComponent|SetMaxWalkSpeed (Variables|Character|GetCharacterMovement) (Utilities|Select :Index Speed :NewEnumerator0 0.0 :NewEnumerator1 2.5e+02 :NewEnumerator2 375.0 :NewEnumerator3 5e+02)))
  (return _output_get))