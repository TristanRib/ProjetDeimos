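; Enemy AI character with health, hit knockback and sight reporting to its Blackboard.
; Damage reduces Health and launches it along the causer's forward vector, then enables mesh physics at zero, though Alive is only reassigned to itself.
; While Alive, PawnSensing writes the seen player's position and sets targetInSight, which a retriggerable delay clears shortly after sightings stop.
; BeginPlay initializes checkedTargetLastSeenPosition as true.
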(event OnSeePawn(PawnSensing)
  (params (Pawn :type Pawn%20Object%20Reference))
  (bind _returnvalue (Utilities|Name|MakeLiteralName "targetInSight"))
  (bind _self self)
  (bind _returnvalue_2 (AI|GetAIController _self))
  (bind _returnvalue_3 (AI|GetBlackboard _returnvalue_2))
  ;[1 1 1] Behavior
  ;;[0.05127 0.05127 0.05127] Vision update
  (if (Variables|Default|GetAlive)
    (Utilities|FlowControl|Sequence
      (:then_0
        (bind _asbp_player (Utilities|Casting|CastToBP_Player Pawn))
        (AI|Components|Blackboard|SetValueasBool _returnvalue_3 _returnvalue true)
        (AI|Components|Blackboard|SetValueasVector _returnvalue_3 (Utilities|Name|MakeLiteralName "targetLastSeenPosition") (Transformation|GetWorldLocation (Variables|/Script/Engine.Character|GetCapsuleComponent _asbp_player))))
      (:then_1
        (Utilities|FlowControl|RetriggerableDelay 0.6)
        (AI|Components|Blackboard|SetValueasBool _returnvalue_3 _returnvalue false)))))

(event EventBeginPlay
  (AI|Components|Blackboard|SetValueasBool (AI|GetBlackboard (AI|GetAIController self)) (Utilities|Name|MakeLiteralName "checkedTargetLastSeenPosition") true))

(event Game|Damage|EventAnyDamage
  (params (Damage :type Float%20%28single-precision%29) (DamageType :type Damage%20Type%20Object%20Reference) (InstigatedBy :type Controller%20Object%20Reference) (DamageCauser :type Actor%20Object%20Reference))
  ;[1 0 0] Health system
  (bind _output_get (Variables|Default|SetHealth (- (Variables|Default|GetHealth) Damage)))
  (if (Utilities|IsValid DamageCauser)
    (Character|LaunchCharacter (+ (* (Transformation|GetActorForwardVector DamageCauser) 2e+02) (* (Transformation|GetActorUpVector) 1e+02)) false false))
  (if (<= _output_get 0.0)
    (Physics|SetSimulatePhysics (Variables|Character|GetMesh) true)
    (Variables|Default|SetAlive (Variables|Default|GetAlive))))

(fn ConstructionScript)