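; Player character Blueprint that handles a stamina-gated melee attack, damage intake and death through health and stamina components.
; The attack input spends stamina and plays a push montage, whose notify sphere-traces forward for pawns, sends them a damage message and reports an AI damage event.
; Reaching zero health ragdolls the mesh and disables input, while getters expose component values.
; Pressing F emits a noise, and stat changes print debug strings.
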(event OnStaminaDecreased(BPC_StaminaSystem)
  (params (info :type S%20Stamina%20Change%20Info%20Structure))
  (Development|PrintString (Utilities|String|Append (Utilities|String|ToString(Float) (.previousvalue info)) " : " (Utilities|String|ToString(Float) (.newvalue info)))))

(event OnHealthUpdated(BPC_HealthSystem)
  (params (Info :type S%20Health%20Change%20Info%20Structure))
  (bind (_previousvalue _newvalue) (Utilities|Struct|BreakS_HealthChangeInfo Info))
  ;[1 0 0] Fight
  (Development|PrintString (Utilities|String|Append "Previous : " (Utilities|String|ToString(Float) _previousvalue) "  " "New : " (Utilities|String|ToString(Float) _newvalue))))

(event OnZeroHealth(BPC_HealthSystem)
  (bind _returnvalue (Game|GetPlayerController 0))
  (bind _mesh (Variables|Character|GetMesh))
  ;[1 0 0] Fight
  ;;[0.15 0.15 0.15 0.5] Commentaire
  (Physics|SetSimulatePhysics _mesh true)
  (Collision|SetCollisionEnabled _mesh "QueryAndPhysics")
  (Input|DisableInput (Pawn|GetController) _returnvalue)
  (Input|DisableInput _returnvalue))

(event Input|EnhancedActionEvents|EnhancedInputActionIA_Attack
  (params (ActionValue :type Boolean) (ElapsedSeconds :type Float%20%28double-precision%29) (TriggeredSeconds :type Float%20%28double-precision%29) (InputAction :type Input%20Action%20Object%20Reference :default "/Game/Blueprints/Inputs/Actions/IA_Attack.IA_Attack"))
  (bind _bpc_staminasystem (Variables|Default|GetBPC_StaminaSystem))
  ;[1 0 0] Fight
  ;;[0.15 0.15 0.15 0.5] Default Attack
  (:Started
    (if (Variables|Default|GetcanAttack)
      (bind _stamina (Default|GetStamina _bpc_staminasystem))
      (if (>= _stamina 2e+01)
        (Default|UpdateStamina _bpc_staminasystem -2e+01)
        (Animation|Montage|PlayMontage (Variables|Character|GetMesh) "/Game/Characters/Mannequins/Animations/Manny/MM_Push_Montage.MM_Push_Montage"
          (:then
            (Variables|Default|SetcanAttack false))
          (:OnCompleted
            (Variables|Default|SetcanAttack true))
          (:OnNotifyBegin
            (CallFunction|ApplyDamage (Utilities|Struct|MakeS_DamageInfo 5e+01 (Utilities|Struct|MakeS_HitType "NewEnumerator1" "NewEnumerator0" 0.0) (Utilities|Struct|MakeS_DamageType "NewEnumerator0" "NewEnumerator0" 0.0)))))))))

(event Input|KeyboardEvents|F
  (params (Key :type Key%20Structure :default "None"))
  (:Pressed
    (Class|Actor|MakeNoise 1.0 self (Transformation|GetActorLocation) 0.0 "None")))

(fn ConstructionScript)

(fn ApplyDamage
  (params (DamageInfo :type S%20Damage%20Info%20Structure))
  (bind _attacktrace (Variables|Default|GetAttackTrace))
  (bind _returnvalue (Transformation|GetWorldLocation _attacktrace))
  (bind (_outhit _returnvalue_2) (Collision|SphereTraceForObjects _returnvalue (+ _returnvalue (* (Math|Vector|GetForwardVector _attacktrace) 1e+02)) 2e+01 (Utilities|Array|MakeArray "ObjectTypeQuery3") false 0 "ForDuration" true "(R=1.000000,G=0.000000,B=0.000000,A=1.000000)" "(R=0.000000,G=1.000000,B=0.000000,A=1.000000)" 1.0))
  (if _returnvalue_2
    (Class|BPIDamageable|ReceiveDamage(Message) (.HitActor (Collision|BreakHitResult _outhit)) DamageInfo)
    (if true
      (Class|AISenseDamage|ReportDamageEvent (.HitActor (Collision|BreakHitResult _outhit)) self (.DamageAmount (Utilities|Struct|BreakS_DamageInfo DamageInfo)) (Transformation|GetActorLocation) "0, 0, 0" "None"))))

(fn GetHealth
  (bind _returnvalue (Default|GetHealth (Variables|Default|GetBPC_HealthSystem)))
  (return _returnvalue))

(fn GetHealthPercentage
  (bind _returnvalue (Default|GetHealthPercentage (Variables|Default|GetBPC_HealthSystem)))
  (return _returnvalue))

(fn GetMaxHealth
  (bind _returnvalue (Default|GetMaxHealth (Variables|Default|GetBPC_HealthSystem)))
  (return _returnvalue))

(fn GetStaminaPercent
  (bind _returnvalue (Default|GetStaminaPercentage (Variables|Default|GetBPC_StaminaSystem)))
  (return _returnvalue))

(fn IsDead
  (bind _returnvalue (Default|IsZeroHealth (Variables|Default|GetBPC_HealthSystem)))
  (return _returnvalue))

(fn ReceiveDamage
  (params (DamageInfo :type S%20Damage%20Info%20Structure))
  (bind _bpc_healthsystem (Variables|Default|GetBPC_HealthSystem))
  (Default|UpdateHealth _bpc_healthsystem (- 0.0 (.DamageAmount (Utilities|Struct|BreakS_DamageInfo DamageInfo))))
  (bind _returnvalue (Default|IsZeroHealth _bpc_healthsystem))
  (return false _returnvalue))