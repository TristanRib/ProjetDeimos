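; BP_PlayController is the player controller that turns Enhanced Input actions into messages for the player pawn.
; On BeginPlay it adds the IMC_Core mapping context and caches the player pawn.
; Look, move and sprint start/stop inputs are forwarded as message calls, leaving the behavior to the pawn.
; A dev T key toggles slow-motion through global time dilation.
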(event Input|EnhancedActionEvents|EnhancedInputActionIA_Move
  (params (ActionValue :type Vector%202D%20Structure) (ElapsedSeconds :type Float%20%28double-precision%29) (TriggeredSeconds :type Float%20%28double-precision%29) (InputAction :type Input%20Action%20Object%20Reference :default "/Game/Characters/Player/Inputs/Actions/IA_Move.IA_Move"))
  ;[0.15 0.15 0.15 0.5] Movements
  (Class|BPIBaseControls|Move(Message) (Variables|Default|GetPlayerPawn) (.x ActionValue) (.y ActionValue)))

(event Input|EnhancedActionEvents|EnhancedInputActionIA_Look
  (params (ActionValue :type Vector%202D%20Structure) (ElapsedSeconds :type Float%20%28double-precision%29) (TriggeredSeconds :type Float%20%28double-precision%29) (InputAction :type Input%20Action%20Object%20Reference :default "/Game/Characters/Player/Inputs/Actions/IA_Look.IA_Look"))
  ;[0.15 0.15 0.15 0.5] Movements
  (Class|BPIBaseControls|Look(Message) (Variables|Default|GetPlayerPawn) (.x ActionValue) (.y ActionValue)))

(event Input|EnhancedActionEvents|EnhancedInputActionIA_Sprint
  (params (ActionValue :type Boolean) (ElapsedSeconds :type Float%20%28double-precision%29) (TriggeredSeconds :type Float%20%28double-precision%29) (InputAction :type Input%20Action%20Object%20Reference :default "/Game/Characters/Player/Inputs/Actions/IA_Sprint.IA_Sprint"))
  (bind _playerpawn (Variables|Default|GetPlayerPawn))
  ;[0.15 0.15 0.15 0.5] Movements
  (:Started
    (Class|BPIBaseControls|StartSprint(Message) _playerpawn))
  (:Completed
    (Class|BPIBaseControls|StopSprint(Message) _playerpawn)))

(event EventBeginPlay
  (bind _self self)
  (bind _returnvalue (PlayerController|LocalPlayerSubsystems|GetEnhancedInputLocalPlayerSubsystem _self))
  ;[0.15 0.15 0.15 0.5] Setup
  (Utilities|IsValid _returnvalue
    (:Is%20Valid
      (Input|AddMappingContext _returnvalue "/Game/Characters/Player/Inputs/IMC_Core.IMC_Core" 0 "(bIgnoreAllPressedKeysUntilRelease=True,bForceImmediately=False,bNotifyUserSettings=False)")
      (Variables|Default|SetPlayerPawn (Game|Player|GetPlayerPawn 0)))))

(event Input|KeyboardEvents|T
  (params (Key :type Key%20Structure :default "None"))
  ;[0.15 0 0.1001 0.5] Dev
  (:Pressed
    (Utilities|FlowControl|FlipFlop
      (:A
        (Utilities|Time|SetGlobalTimeDilation 0.1))
      (:B
        (Utilities|Time|SetGlobalTimeDilation 1.0)))))

(fn ConstructionScript)