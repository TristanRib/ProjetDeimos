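; BP_Enemy_Melee is a melee enemy NPC that supplies a close-range default attack on top of its parent enemy class.
; DefaultAttack plays a push montage, and its notify triggers a short forward sphere trace for pawns from the AttackTrace component, with debug drawing enabled.
; A hit sends a damage message to the actor, and montage completion or interruption signals attack end.
; GetPatrolRoute is empty.
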(event EventBeginPlay
  (|CallParentFunction))

(event EventDefaultAttack
  (bind _attacktrace (Variables|Default|GetAttackTrace))
  (bind _returnvalue (Transformation|GetWorldLocation _attacktrace))
  ;[0.05127 0.05127 0.05127] Attack
  (Animation|Montage|PlayMontage (Variables|Character|GetMesh) "/Game/Characters/Mannequins/Animations/Manny/MM_Push_Montage.MM_Push_Montage"
    (:OnCompleted
      (Default|CallOnAttackEnd :!label _label))
    (:OnInterrupted
      (goto _label))
    (:OnNotifyBegin
      (bind (_outhit _returnvalue_2) (Collision|SphereTraceForObjects _returnvalue (+ _returnvalue (* (Math|Vector|GetForwardVector _attacktrace) 1e+02)) 2e+01 (Utilities|Array|MakeArray "ObjectTypeQuery3") false 0 "ForDuration" true "(R=1.000000,G=0.000000,B=0.000000,A=1.000000)" "(R=0.000000,G=1.000000,B=0.000000,A=1.000000)" 1.0))
      (if _returnvalue_2
        (Class|BPIDamageable|ReceiveDamage(Message) (.HitActor (Collision|BreakHitResult _outhit)) (Utilities|Struct|MakeS_DamageInfo 2e+01 (Utilities|Struct|MakeS_HitType "NewEnumerator0" "NewEnumerator0" 0.0) (Utilities|Struct|MakeS_DamageType "NewEnumerator0" "NewEnumerator0" 0.0)))))))

(fn ConstructionScript
  (|CallParentFunction))

(fn GetPatrolRoute
  (return 0))