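; BP_Enemy_Range is a ranged enemy NPC Blueprint that supplies its own attack, movement speeds and preferred combat distances.
; DefaultAttack plays a push montage on the mesh and signals OnAttackEnd whether it completes or is interrupted, with no projectile or damage logic here.
; SetMovementSpeed maps a movement state to max walk speed, and GetIdealRange reports the same distance for attacking and defending.
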(event EventBeginPlay
  (|CallParentFunction))

(event EventDefaultAttack
  ;[0.05127 0.05127 0.05127] Attack
  (Animation|Montage|PlayMontage (Variables|Character|GetMesh) "/Game/Characters/Mannequins/Animations/Manny/MM_Push_Montage.MM_Push_Montage"
    (:OnCompleted
      _)
    (:OnInterrupted
      _))
  (Default|CallOnAttackEnd))

(fn ConstructionScript
  (|CallParentFunction))

(fn SetMovementSpeed
  (params (Speed :type E_MovementSpeed%20Enum :default "NewEnumerator0"))
  (Variables|/Script/Engine.CharacterMovementComponent|SetMaxWalkSpeed (Variables|Character|GetCharacterMovement) (Utilities|Select :Index Speed :NewEnumerator0 0.0 :NewEnumerator4 1.5e+02 :NewEnumerator1 2.5e+02 :NewEnumerator2 375.0 :NewEnumerator3 5e+02))
  (return 0.0))

(fn GetIdealRange
  (return 7.5e+02 7.5e+02))