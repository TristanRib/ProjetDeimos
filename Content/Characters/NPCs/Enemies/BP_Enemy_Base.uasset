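; BP_Enemy_Base is an enemy character base with health, damage handling and a floating health bar that faces the player camera.
; Health queries and incoming damage go through BPC_HealthSystem; zero health ragdolls the mesh, disables capsule collision, hides the bar and sets AIC_Enemy_Base to dead.
; It also exposes patrol route, attack and defend radii, and enum-driven walk speed.
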(event OnZeroHealth(BPC_HealthSystem)
  (bind _mesh (Variables|Character|GetMesh))
  ;[1 0 0] Health system
  (Physics|SetSimulatePhysics _mesh true)
  (Collision|SetCollisionEnabled _mesh "QueryAndPhysics")
  (Default|SetStateasDead (Variables|Default|GetAIController))
  (Collision|SetCollisionEnabled (Variables|Collision|GetCapsuleComponent) "NoCollision")
  (Rendering|SetVisibility (Variables|Default|GetHealthBar) false false))

(event EventBeginPlay
  ;[0.15 0.15 0.15 0.5] Commentaire
  (bind _asaic_enemy_base (Utilities|Casting|CastToAIC_Enemy_Base (AI|GetAIController self)))
  (Variables|Default|SetAIController _asaic_enemy_base)
  (bind _returnvalue (UserInterface|CreateWidget "/Game/Systems/HealthSystem/Widgets/W_HealthBar.W_HealthBar_C" 0 self))
  (UserInterface|SetWidget (Variables|Default|GetHealthBar) _returnvalue))

(event EventTick
  (params (DeltaSeconds :type Float%20%28single-precision%29))
  (bind _healthbar (Variables|Default|GetHealthBar))
  (Transformation|SetWorldRotation _healthbar (Math|Rotator|FindLookatRotation (Transformation|GetWorldLocation _healthbar) (Transformation|GetWorldLocation (Variables|/Script/Engine.Actor|GetRootComponent (Game|GetPlayerCameraManager 0)))) false false))

(fn ConstructionScript)

(fn GetHealth
  (bind _returnvalue (Default|GetHealth (Variables|Default|GetBPC_HealthSystem)))
  (return _returnvalue))

(fn GetHealthPercentage
  (bind _returnvalue (Default|GetHealthPercentage (Variables|Default|GetBPC_HealthSystem)))
  (return _returnvalue))

(fn GetIdealRange
  (return 1.5e+02 3.5e+02))

(fn GetMaxHealth
  (bind _returnvalue (Default|GetMaxHealth (Variables|Default|GetBPC_HealthSystem)))
  (return _returnvalue))

(fn GetPatrolRoute
  (return (Variables|AI|GetPatrol%20Route)))

(fn IsDead
  (bind _returnvalue (Default|IsZeroHealth (Variables|Default|GetBPC_HealthSystem)))
  (return _returnvalue))

(fn ReceiveDamage
  (params (DamageInfo :type S%20Damage%20Info%20Structure))
  (bind _bpc_healthsystem (Variables|Default|GetBPC_HealthSystem))
  (Default|UpdateHealth _bpc_healthsystem (- 0.0 (.DamageAmount (Utilities|Struct|BreakS_DamageInfo DamageInfo))))
  (bind _returnvalue (Default|IsZeroHealth _bpc_healthsystem))
  (return false _returnvalue))

(fn SetMovementSpeed
  (params (Speed :type E_MovementSpeed%20Enum :default "NewEnumerator0"))
  (bind _output_get (Variables|/Script/Engine.CharacterMovementComponent|SetMaxWalkSpeed (Variables|Character|GetCharacterMovement) (Utilities|Select :Index Speed :NewEnumerator0 0.0 :NewEnumerator4 1.5e+02 :NewEnumerator1 2.5e+02 :NewEnumerator2 375.0 :NewEnumerator3 5e+02)))
  (return _output_get))