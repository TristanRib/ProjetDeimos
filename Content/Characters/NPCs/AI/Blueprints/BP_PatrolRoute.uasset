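; BP_PatrolRoute is an NPC patrol route that uses a spline's points as waypoints.
; It stores the current point index and a travel direction, and GetSplinePointWorldPosition returns that point's world location.
; IncrementPatrol steps the index by the direction and flips the direction at the first and last points, so the route runs back and forth rather than looping.
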(event Custom|IncrementPatrol
  (bind _output_get (Variables|Default|SetPatrolPointIndex (+ (Variables|Default|GetPatrolPointIndex) (Variables|Default|GetPatrolDirection))))
  (if (== _output_get (- (Spline|GetNumberOfSplinePoints (Variables|Default|GetPatrolRoute)) 1))
    (Variables|Default|SetPatrolDirection -1)
    (elif (== (Variables|Default|GetPatrolPointIndex) 0)
      (Variables|Default|SetPatrolDirection 1))))

(fn ConstructionScript)

(fn GetSplinePointWorldPosition
  (return (Spline|GetLocationatSplinePoint (Variables|Default|GetPatrolRoute) (Variables|Default|GetPatrolPointIndex) "World")))