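; BP_Enemy is an AI enemy character that wanders, chases the player on sight and takes damage.
; Wander and chase each loop AI Move To with pauses, targeting random reachable points or the player.
; Pawn sensing triggers the chase, and a retriggerable delay sends it to the last seen location once sightings stop, then back to wandering.
; Damage launches it along the causer's forward vector and ragdolls the mesh at zero health.
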(event OnSeePawn(PawnSensing)
  (params (Pawn :type Pawn%20Object%20Reference))
  ;[1 1 1] Movements
  ;;[1 1 1] Behavior
  (Utilities|FlowControl|Sequence
    (:then_0
      (Utilities|Casting|CastToBP_Player Pawn)
      (CallFunction|ChasePlayer))
    (:then_1
      (Utilities|FlowControl|RetriggerableDelay 1.0)
      (AI|AIMoveTo self (Variables|Default|GetLastSeenLocation) 0 5.0 false
        (:OnSuccess
          (Utilities|FlowControl|Delay 4.0)
          (CallFunction|Wander))))))

(event Custom|ChasePlayer
  (bind _returnvalue (Game|GetPlayerCharacter 0))
  ;[1 1 1] Movements
  ;;[1 1 1] Movement chase system
  (Variables|Default|SetLastSeenLocation (Transformation|GetWorldLocation (Variables|/Script/Engine.Character|GetCapsuleComponent _returnvalue)))
  (AI|AIMoveTo self "0, 0, 0" _returnvalue 5.0 false :!label _label
    (:OnSuccess
      (Utilities|FlowControl|Delay 1.0)
      (goto _label))))

(event Custom|Wander
  ;[1 1 1] Movements
  ;;[1 1 1] Movement wander system
  (AI|AIMoveTo self (.RandomLocation (AI|Navigation|GetRandomReachablePointinRadius (Transformation|GetActorLocation) 1e+03 0 0)) 0 5.0 false :!label _label
    (:OnSuccess
      (Utilities|FlowControl|Delay 2.0)
      (goto _label))))

(event Game|Damage|EventAnyDamage
  (params (Damage :type Float%20%28single-precision%29) (DamageType :type Damage%20Type%20Object%20Reference) (InstigatedBy :type Controller%20Object%20Reference) (DamageCauser :type Actor%20Object%20Reference))
  ;[1 0 0] Health system
  (bind _output_get (Variables|Default|SetHealth (- (Variables|Default|GetHealth) Damage)))
  (if (Utilities|IsValid DamageCauser)
    (Character|LaunchCharacter (+ (* (Transformation|GetActorForwardVector DamageCauser) 2e+02) (* (Transformation|GetActorUpVector) 1e+02)) false false))
  (if (<= _output_get 0.0)
    (Physics|SetSimulatePhysics (Variables|Character|GetMesh) true)))

(event EventBeginPlay
  (CallFunction|Wander))

(fn ConstructionScript)